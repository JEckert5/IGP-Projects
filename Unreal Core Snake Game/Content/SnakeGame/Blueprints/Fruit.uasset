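; Fruit is a collectible actor for a Snake game that the player eats to trigger the next fruit spawn.
; Its PlayerOverlap event calls EatFruit on the player, then asks the SnakeGameMode to spawn a new fruit and destroys itself.
; If the game mode cast fails, the fruit is not destroyed.
; BeginPlay, overlap and Tick events are unused stubs.
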(event EventBeginPlay
  (|CallParentFunction) ; This node is disabled and will not be called.\nDrag off pins to build functionality.
)

(event Collision|EventActorBeginOverlap
  (params (OtherActor :type Actor%20Object%20Reference))
  (|CallParentFunction OtherActor) ; This node is disabled and will not be called.\nDrag off pins to build functionality.
)

(event EventTick
  (params (DeltaSeconds :type Float%20%28single-precision%29))
  (|CallParentFunction DeltaSeconds) ; This node is disabled and will not be called.\nDrag off pins to build functionality.
)

(event EventPlayerOverlap
  (params (Player :type BP%20Snake%20Head%20Object%20Reference))
  (Default|EatFruit Player)
  (bind _assnake_game_mode (Utilities|Casting|CastToSnakeGameMode (Game|GetGameMode)))
  (Default|SpawnFruit _assnake_game_mode)
  (Actor|DestroyActor))

(fn ConstructionScript
  (|CallParentFunction))